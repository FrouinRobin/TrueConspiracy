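; BP_MenInBlack is the Men In Black Face Blueprint, triggering that face's effects at set game timings.
; Six events cover placement, each turn, and the start and end of turns and phases.
; Each event searches the FaceEffect list for the matching effect-type class and calls DoEffect if one is valid.
; The graph holds no effect logic of its own, delegating it all to those effect objects.
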(event EventOnFaceEachTurn
  (bind _returnvalue (Class|TCFace|FindEffectOfType (Variables|Default|GetFaceEffect) "/Game/TrueConspiracy/EffectType/BP_EffectTypeEachTurn.BP_EffectTypeEachTurn_C"))
  (Utilities|IsValid _returnvalue
    (:Is%20Valid
      (Class|TCEffectType|DoEffect _returnvalue))))

(event EventOnFaceEndPhase
  (bind _returnvalue (Class|TCFace|FindEffectOfType (Variables|Default|GetFaceEffect) "/Game/TrueConspiracy/EffectType/BP_EffectTypeEndPhase.BP_EffectTypeEndPhase_C"))
  (Utilities|IsValid _returnvalue
    (:Is%20Valid
      (Class|TCEffectType|DoEffect _returnvalue))))

(event EventOnFaceEndTurn
  (bind _returnvalue (Class|TCFace|FindEffectOfType (Variables|Default|GetFaceEffect) "/Game/TrueConspiracy/EffectType/BP_EffectTypeEndTurn.BP_EffectTypeEndTurn_C"))
  (Utilities|IsValid _returnvalue
    (:Is%20Valid
      (Class|TCEffectType|DoEffect _returnvalue))))

(event EventOnFacePlace
  (bind _returnvalue (Class|TCFace|FindEffectOfType (Variables|Default|GetFaceEffect) "/Game/TrueConspiracy/EffectType/BP_EffectTypeOnPlace.BP_EffectTypeOnPlace_C"))
  (Utilities|IsValid _returnvalue
    (:Is%20Valid
      (Class|TCEffectType|DoEffect _returnvalue))))

(event EventOnFaceStartPhase
  (bind _returnvalue (Class|TCFace|FindEffectOfType (Variables|Default|GetFaceEffect) "/Game/TrueConspiracy/EffectType/BP_EffectTypeStartPhase.BP_EffectTypeStartPhase_C"))
  (Utilities|IsValid _returnvalue
    (:Is%20Valid
      (Class|TCEffectType|DoEffect _returnvalue))))

(event EventOnFaceStartTurn
  (bind _returnvalue (Class|TCFace|FindEffectOfType (Variables|Default|GetFaceEffect) "/Game/TrueConspiracy/EffectType/BP_EffectTypeStartTurn.BP_EffectTypeStartTurn_C"))
  (Utilities|IsValid _returnvalue
    (:Is%20Valid
      (Class|TCEffectType|DoEffect _returnvalue))))