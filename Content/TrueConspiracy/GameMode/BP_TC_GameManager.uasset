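; Game mode for True Conspiracy that assigns joining players to pawns and starts a two-player best-of-three match.
; On PostLogin it looks for an unpossessed BP_PlayerPawn, has the new player possess it, records it, and calls StartGame once two are logged.
; BeginPlay also caches the BP_TC_Plate and calls StartGame directly with the first two pawns in the level, independent of logins.
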(event EventTick
  (params (DeltaSeconds :type Float%20%28single-precision%29)))

(event EventPostLogin
  (params (NewPlayer :type Player%20Controller%20Object%20Reference))
  (bind _playerlogged (Variables|Default|GetPlayerLogged))
  (Development|PrintText "OnPostLogin")
  (bind _outactors (Actor|GetAllActorsOfClass "/Game/TrueConspiracy/Player/BP_PlayerPawn.BP_PlayerPawn_C"))
  (bind _array_element (Utilities|Array|ForEachLoopwithBreak _outactors :!label _label)
    (:LoopBody
      (if (not (Variables|/Script/TrueConspiracy.TC_Player|GetIsPossessed _array_element))
        (goto _label Break)))
    (:Completed
      (Pawn|Possess NewPlayer _array_element)
      (Variables|/Script/TrueConspiracy.TC_Player|SetIsPossessed _array_element true)
      (Utilities|Array|AddUnique _playerlogged _array_element)
      (if (== (Utilities|Array|Length _playerlogged) 2)
        (Class|TCGameManager|StartGame "BO3" _playerlogged)))))

(event EventBeginPlay
  (bind _outactors (Actor|GetAllActorsOfClass "/Game/TrueConspiracy/Player/BP_PlayerPawn.BP_PlayerPawn_C"))
  (bind _returnvalue (Actor|GetActorOfClass "/Game/TrueConspiracy/Board/BP_TC_Plate.BP_TC_Plate_C"))
  (Variables|Default|SetPlate _returnvalue)
  (Class|TCGameManager|StartGame "BO3" (Utilities|Array|MakeArray (Utilities|Array|Get(acopy) _outactors) (Utilities|Array|Get(acopy) _outactors 1))))

(fn ConstructionScript)