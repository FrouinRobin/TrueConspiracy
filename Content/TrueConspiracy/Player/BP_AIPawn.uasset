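; AI pawn for the True Conspiracy card game, reacting to card selection, player state and phase changes.
; On BeginPlay it sets the camera aspect ratio, finds its board through the plate and draws the opening hand.
; State changes ease the camera anchor to mapped transforms and force target selection when cards await targets and its board holds several cards.
; Selection nudges card anchors; phase changes rotate the player's cards.
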(event EventBeginPlay
  (bind _self self)
  (Class|CameraComponent|SetAspectRatio (Variables|Default|GetPlayerCamera) (Class|WidgetLayoutLibrary|GetViewportScale))
  (bind _returnvalue (Actor|GetActorOfClass "/Game/TrueConspiracy/Board/BP_TC_Plate.BP_TC_Plate_C"))
  (bind _returnvalue_2 (Class|TCPlate|GetBoardbyPlayer _returnvalue _self))
  (bind _returnvalue_3 (Class|TCBoard|GetBoardPlayer _returnvalue_2))
  (if (== _returnvalue_3 _self)
    (Class|TCBoard|OnDrawNumberOfCard _returnvalue_2 5)))

(event Collision|EventActorBeginOverlap
  (params (OtherActor :type Actor%20Object%20Reference)))

(event EventTick
  (params (DeltaSeconds :type Float%20%28single-precision%29)))

(event EventOnStateChange
  (params (newState :type ETC_PlayerState%20Enum :default "SELECTHAND") (oldState :type ETC_PlayerState%20Enum :default "SELECTHAND"))
  (bind _playertransform (Variables|Default|GetPlayerTransform))
  (bind (_value _returnvalue) (Utilities|Map|Find _playertransform newState))
  (bind (_location _rotation) (Math|Transform|BreakTransform _value))
  (Utilities|FlowControl|Sequence
    (:then_0
      (if (Math|Boolean|ANDBoolean (>= (Utilities|Array|Length (Class|TCPlayer|GetCardsWaitingTargetList)) 1) (Utilities|Enum|NotEqual(Enum) newState "SELECTTARGET") (CallFunction|CanTargetbeChoosen))
        (Class|TCPlayer|SetPlayerState "SELECTTARGET")))
    (:then_1
      (if _returnvalue
        (Components|MoveComponentTo (Variables|Default|GetCameraAnchor) _location _rotation true true 1.0 true)))))

(event EventOnChangePhaseState
  (params (newPhaseState :type ETC_PhaseState%20Enum :default "Attack"))
  (bind _returnvalue (Class|TCPlayer|GetAllPlayerCard true))
  (if (> (Utilities|Array|Length _returnvalue) 0)
    (for _array_element _returnvalue
      (Class|TCCard|OnCardRotate _array_element))))

(event EventOnSelectCard
  (params (card :type TC%20Card%20Object%20Reference) (oldCard :type TC%20Card%20Object%20Reference))
  (Utilities|FlowControl|Sequence
    (:then_0
      (if (Utilities|IsValid card)
        (Transformation|AddLocalOffset (Variables|/Script/TrueConspiracy.TC_Card|GetCardAnchor card) "-10.000000,0.000000,0.000000" true false)))
    (:then_1
      (if (Utilities|IsValid oldCard)
        (Transformation|AddLocalOffset (Variables|/Script/TrueConspiracy.TC_Card|GetCardAnchor oldCard) "10.000000,0.000000,-0.000000" true false)))))

(fn ConstructionScript)

(fn CanTargetbeChoosen
  (bind _returnvalue (Class|TCPlayer|GetPlayerBoard))
  (bind _returnvalue_2 (Class|TCBoard|GetBoardSlots _returnvalue))
  (for _array_element _returnvalue_2
    (bind _returnvalue_3 (Class|TCBoardSlot|GetBoardSlotSlots _array_element))
    (for _array_element_2 _returnvalue_3
      (bind _returnvalue_4 (Class|TCSlot|HasCard _array_element_2))
      (if _returnvalue_4
        (Math|Integer|IncrementInt (LocalVariables|GetCount)))))
  (return (> (LocalVariables|GetCount) 1)))

(fn GetPawnController
  (bind _astc_player_controller (Utilities|Casting|CastToTC_PlayerController (Pawn|GetController))
    (:then
      _)
    (:CastFailed
      _))
  (return _astc_player_controller))