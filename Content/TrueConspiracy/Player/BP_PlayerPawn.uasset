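; BP_PlayerPawn is the player pawn for a card game, handling camera setup, the opening draw and card selection feedback.
; On BeginPlay it sets the camera aspect ratio from the viewport scale, finds its board through BP_TC_Plate and, if it owns that board, draws five cards.
; OnSelectCard nudges the newly selected card along its local Y axis and moves the previous one back, using swept offsets.
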(event EventBeginPlay
  (bind _self self)
  (Class|CameraComponent|SetAspectRatio (Variables|Default|Get_playerCamera) (Class|WidgetLayoutLibrary|GetViewportScale))
  (bind _returnvalue (Actor|GetActorOfClass "/Game/TrueConspiracy/Board/BP_TC_Plate.BP_TC_Plate_C"))
  (bind _returnvalue_2 (Class|TCPlate|GetBoardbyPlayer _returnvalue _self))
  (bind _returnvalue_3 (Class|TCBoard|GetBoardPlayer _returnvalue_2))
  (if (== _returnvalue_3 _self)
    (Class|TCBoard|OnDrawNumberOfCard _returnvalue_2 5)))

(event Collision|EventActorBeginOverlap
  (params (OtherActor :type Actor%20Object%20Reference)))

(event EventTick
  (params (DeltaSeconds :type Float%20%28single-precision%29)))

(event EventOnSelectCard
  (params (card :type TC%20Card%20Object%20Reference) (oldCard :type TC%20Card%20Object%20Reference))
  (Utilities|FlowControl|Sequence
    (:then_0
      (if (Utilities|IsValid card)
        (Transformation|AddActorLocalOffset card "0.000000,10.000000,0.000000" true false)))
    (:then_1
      (if (Utilities|IsValid oldCard)
        (Transformation|AddActorLocalOffset oldCard "0.000000,-10.000000,0.000000" true false)))))

(fn ConstructionScript)