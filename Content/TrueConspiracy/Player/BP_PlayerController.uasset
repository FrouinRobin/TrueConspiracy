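; Player controller for a card game that turns touch hits into card selection, drawing and playing.
; OnTouchTriggered switches on pawn state and casts the hit actor to card, slot or draw deck.
; Idle selects hand cards, draws from the player's own deck, deselects on empty hits, or enters slot selection when a slot is hit with a card selected.
; Selecting Slot plays that card on the hit slot; disconnected older versions remain unused.
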(event EventBeginPlay)

(event EventTick
  (params (DeltaSeconds :type Float%20%28single-precision%29)))

(event EventOnInputStart
  (params (EnhancedInputComponent :type Enhanced%20Input%20Component%20Object%20Reference)))

(event EventOnTouchReleased)

(event EventOnTouchTriggered
  (params (hit :type Hit%20Result%20Structure) (didHit :type Boolean))
  (bind _object (CallFunction|GetEssentialfromHit hit))
  (bind _returnvalue (Class|TCPlayerController|GetMyPawn))
  (bind _returnvalue_2 (Class|TCPlayerController|GetMyPawn))
  (bind _returnvalue_3 (Class|TCPlayerController|GetMyPawn))
  (bind _returnvalue_4 (Class|TCPlayerController|GetMyPawn))
  (bind _returnvalue_5 (Class|TCPlayer|GetSelectedCard _returnvalue_3))
  (Variables|Default|SetHitCache didHit)
  (switch Utilities|FlowControl|Switch|SwitchonETC_PlayerState (Class|TCPlayer|GetState (Class|TCPlayerController|GetMyPawn))
    (:SELECTHAND
      ;[1 0 0.2601 0.5] Select a card
      (if (Variables|Default|GetHitCache)
        (bind _astc_card (Utilities|Casting|CastToTC_Card _object)
          (:then
            (bind _returnvalue_6 (Class|TCPlayer|GetHand _returnvalue_2))
            (if (Utilities|Array|ContainsItem _returnvalue_6 _astc_card)
              (Class|TCPlayer|SetSelectedCard _returnvalue_2 _astc_card)))
          (:CastFailed
            (Utilities|Casting|CastToTC_Slot _object
              (:then
                (if (Utilities|IsValid (Class|TCPlayer|GetSelectedCard _returnvalue_2))
                  (Class|TCPlayer|SetState _returnvalue_2 "SELECTSLOT")))
              (:CastFailed
                ;[0.15 0.15 0.15 0.5] Select the Deck
                (bind _astc_draw_deck (Utilities|Casting|CastToTC_DrawDeck _object)
                  (:then
                    (bind _returnvalue_7 (Class|TCDrawDeck|GetDrawDeckBoard _astc_draw_deck))
                    (bind _returnvalue_8 (Class|TCBoard|GetBoardPlayer _returnvalue_7))
                    (if (== _returnvalue_8 _returnvalue_4)
                      (bind _returnvalue_9 (Class|TCBoard|GetBoardDraw _returnvalue_7))
                      (bind _returnvalue_10 (Class|TCDrawDeck|GetDrawDeckGameFirstCard _returnvalue_9))
                      (Class|TCPlayer|AddCardtoHand _returnvalue_4 (Utilities|GetClass _returnvalue_10))))
                  (:CastFailed
                    ;[1 0.15 0.15 0.5] Click on nothing - Deselect the card
                    (if (Utilities|IsValid (Class|TCPlayer|GetSelectedCard _returnvalue)) :!label _label
                      (Class|TCPlayer|SetSelectedCard _returnvalue))))))))
        (else
          (goto _label))))
    (:SELECTSLOT
      ;[0.15 1 1 0.5] Choosing Slot
      (if (Variables|Default|GetHitCache)
        (bind _astc_slot (Utilities|Casting|CastToTC_Slot _object))
        (if (Utilities|IsValid _returnvalue_5)
          (Class|TCPlayer|PlayCard _returnvalue_3 _returnvalue_5 _astc_slot)
          (Class|TCPlayer|SetState _returnvalue_3 "SELECTHAND"))))))

(event EventOnTouchHold
  (params (hit :type Hit%20Result%20Structure) (didHit :type Boolean)))

(fn ConstructionScript)

(fn GetEssentialfromHit
  (params (hit :type Hit%20Result%20Structure))
  (bind (_bblockinghit _binitialoverlap _time _distance _location _impactpoint _normal _impactnormal _physmat _hitactor) (Collision|BreakHitResult hit))
  (return _hitactor _location _distance))