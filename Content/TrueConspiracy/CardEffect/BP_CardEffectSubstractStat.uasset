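; Card effect that subtracts configured Score and Mana values from cards when activated.
; Activate dispatches on EffectLocalisation to gather the caster's lane, both boards or each slot pair, then TargetType selects Ally, Enemy, All or AllExceptSelf logic.
; The TargetCardAttribute check only breaks its loop, so it filters nothing.
; Self, Player Hand and Player handlers are empty stubs, and TargetLogic is never called here.
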(event EventActivate
  (params (Caster :type TC%20Card%20Object%20Reference))
  (switch Utilities|FlowControl|Switch|SwitchonETC_EffectLocalisation (Variables|Default|GetEffectLocalisation)
    (:Land
      (CallFunction|LandLogic Caster))
    (:Board
      (CallFunction|BoardLogic Caster))
    (:Plate
      (CallFunction|PlateLogic Caster))
    (:PlayerHand
      (CallFunction|PlayerHandLogic Caster))
    (:Player
      (CallFunction|PlayerLogic Caster))))

(fn AllyLogic
  (params (Caster :type TC%20Card%20Object%20Reference) (AllyBoardSlot :type TC%20Board%20Slot%20Object%20Reference) (EnemyBoardSlot :type TC%20Board%20Slot%20Object%20Reference) (AllyBoard :type TC%20Board%20Object%20Reference) (EnemyBoard :type TC%20Board%20Object%20Reference) (AllyPlayerHand :type Array%20of%20TC%20Card%20Object%20References) (EnemyPlayerHand :type Array%20of%20TC%20Card%20Object%20References))
  (Utilities|IsValid AllyBoardSlot
    (:Is%20Valid
      (bind _returnvalue (Class|TCBoardSlot|GetBoardSlotSlots AllyBoardSlot))
      (for _array_element _returnvalue
        (bind _returnvalue_2 (Class|TCSlot|GetSlotCard _array_element))
        (Utilities|IsValid _returnvalue_2
          (:Is%20Valid
            (if (!= _returnvalue_2 Caster)
              (bind _returnvalue_3 (Class|TCCard|GetCardAttribute _returnvalue_2))
              (bind _array_element_2 (Utilities|Array|ForEachLoopwithBreak _returnvalue_3 :!label _label)
                (:LoopBody
                  (if (Utilities|Array|ContainsItem (Variables|Default|GetTargetCardAttribute) _array_element_2)
                    (goto _label Break)))
                (:Completed
                  (for _array_element_3 (Variables|Default|GetDataType)
                    (switch Utilities|FlowControl|Switch|SwitchonETC_DataType (.DataType (Utilities|Struct|BreakTC_DataTypeStruct _array_element_3))
                      (:Score
                        (bind _returnvalue_4 (Class|TCCard|GetCardCurrentScore _returnvalue_2))
                        (Class|TCCard|SetCardCurrentScore _returnvalue_2 (- _returnvalue_4 (Math|Conversions|ToFloat(Byte) (.StatValue (Utilities|Struct|BreakTC_DataTypeStruct _array_element_3))))))
                      (:Mana
                        (bind _returnvalue_5 (Class|TCCard|GetCardCurrentMana _returnvalue_2))
                        (Class|TCCard|SetCardCurrentMana _returnvalue_2 (- _returnvalue_5 (Math|Conversions|ToFloat(Byte) (.StatValue (Utilities|Struct|BreakTC_DataTypeStruct _array_element_3)))))))))))))))
    (:Is%20Not%20Valid
      (Utilities|IsValid AllyBoard
        (:Is%20Valid
          (bind _returnvalue_6 (Class|TCBoard|GetBoardSlots AllyBoard))
          (for _array_element_4 _returnvalue_6
            (bind _returnvalue_7 (Class|TCBoardSlot|GetBoardSlotSlots _array_element_4))
            (for _array_element_5 _returnvalue_7
              (bind _returnvalue_8 (Class|TCSlot|GetSlotCard _array_element_5))
              (Utilities|IsValid _returnvalue_8
                (:Is%20Valid
                  (if (!= _returnvalue_8 Caster)
                    (bind _returnvalue_9 (Class|TCCard|GetCardAttribute _returnvalue_8))
                    (bind _array_element_6 (Utilities|Array|ForEachLoopwithBreak _returnvalue_9 :!label _label_2)
                      (:LoopBody
                        (if (Utilities|Array|ContainsItem (Variables|Default|GetTargetCardAttribute) _array_element_6)
                          (goto _label_2 Break)))
                      (:Completed
                        (for _array_element_7 (Variables|Default|GetDataType)
                          (switch Utilities|FlowControl|Switch|SwitchonETC_DataType (.DataType (Utilities|Struct|BreakTC_DataTypeStruct _array_element_7))
                            (:Score
                              (bind _returnvalue_10 (Class|TCCard|GetCardCurrentScore _returnvalue_8))
                              (Class|TCCard|SetCardCurrentScore _returnvalue_8 (- _returnvalue_10 (Math|Conversions|ToFloat(Byte) (.StatValue (Utilities|Struct|BreakTC_DataTypeStruct _array_element_7))))))
                            (:Mana
                              (bind _returnvalue_11 (Class|TCCard|GetCardCurrentMana _returnvalue_8))
                              (Class|TCCard|SetCardCurrentMana _returnvalue_8 (- _returnvalue_11 (Math|Conversions|ToFloat(Byte) (.StatValue (Utilities|Struct|BreakTC_DataTypeStruct _array_element_7))))))))))))))))
        (:Is%20Not%20Valid
          (if (> (Utilities|Array|Length AllyPlayerHand) 0)
            (for _array_element_8 AllyPlayerHand
              (Utilities|IsValid _array_element_8
                (:Is%20Valid
                  (bind _returnvalue_12 (Class|TCCard|GetCardAttribute _array_element_8))
                  (bind _array_element_9 (Utilities|Array|ForEachLoopwithBreak _returnvalue_12 :!label _label_3)
                    (:LoopBody
                      (if (Utilities|Array|ContainsItem (Variables|Default|GetTargetCardAttribute) _array_element_9)
                        (goto _label_3 Break)))
                    (:Completed
                      (for _array_element_10 (Variables|Default|GetDataType)
                        (switch Utilities|FlowControl|Switch|SwitchonETC_DataType (.DataType (Utilities|Struct|BreakTC_DataTypeStruct _array_element_10))
                          (:Score
                            (bind _returnvalue_13 (Class|TCCard|GetCardCurrentScore _array_element_8))
                            (Class|TCCard|SetCardCurrentScore _array_element_8 (- _returnvalue_13 (Math|Conversions|ToFloat(Byte) (.StatValue (Utilities|Struct|BreakTC_DataTypeStruct _array_element_10))))))
                          (:Mana
                            (bind _returnvalue_14 (Class|TCCard|GetCardCurrentMana _array_element_8))
                            (Class|TCCard|SetCardCurrentMana _array_element_8 (- _returnvalue_14 (Math|Conversions|ToFloat(Byte) (.StatValue (Utilities|Struct|BreakTC_DataTypeStruct _array_element_10)))))))))))))))))))

(fn LandLogic
  (params (Caster :type TC%20Card%20Object%20Reference))
  (bind _returnvalue (Class|TCCard|GetSlot Caster))
  (bind _returnvalue_2 (Class|TCSlot|GetSlotBoardSlot _returnvalue))
  (bind _returnvalue_3 (Class|TCBoardSlot|GetBoardSlotOppositeBoard _returnvalue_2))
  (switch Utilities|FlowControl|Switch|SwitchonETC_TargetType (Variables|Default|GetTargetType)
    (:Self
      (CallFunction|SelfLogic))
    (:Ally
      (CallFunction|AllyLogic Caster _returnvalue_2 _returnvalue_3))
    (:Enemy
      (CallFunction|EnemyLogic Caster _returnvalue_2 _returnvalue_3))
    (:AllExceptSelf
      (CallFunction|AllExceptSelfLogic Caster _returnvalue_2 _returnvalue_3))
    (:All
      (CallFunction|AllLogic Caster _returnvalue_2 _returnvalue_3))))

(fn BoardLogic
  (params (Caster :type TC%20Card%20Object%20Reference))
  (bind _returnvalue (Class|TCCard|GetPlayer Caster))
  (bind _returnvalue_2 (Class|TCPlayer|GetPlayerBoard _returnvalue))
  (bind _returnvalue_3 (Class|TCBoard|GetBoardSlots _returnvalue_2))
  (bind _returnvalue_4 (Class|TCBoardSlot|GetBoardSlotOppositeBoard (Utilities|Array|Get(acopy) _returnvalue_3)))
  (bind _returnvalue_5 (Class|TCBoardSlot|GetBoardSlotBoard _returnvalue_4))
  (switch Utilities|FlowControl|Switch|SwitchonETC_TargetType (Variables|Default|GetTargetType)
    (:Self
      (CallFunction|SelfLogic))
    (:Ally
      (CallFunction|AllyLogic 0 0 0 _returnvalue_2 _returnvalue_5))
    (:Enemy
      (CallFunction|EnemyLogic 0 0 0 _returnvalue_2 _returnvalue_5))
    (:AllExceptSelf
      (CallFunction|AllExceptSelfLogic 0 0 0 _returnvalue_2 _returnvalue_5))
    (:All
      (CallFunction|AllLogic 0 0 0 _returnvalue_2 _returnvalue_5))))

(fn PlateLogic
  (params (Caster :type TC%20Card%20Object%20Reference))
  (bind _returnvalue (Class|TCCard|GetSlot Caster))
  (bind _returnvalue_2 (Class|TCSlot|GetSlotBoardSlot _returnvalue))
  (bind _returnvalue_3 (Class|TCBoardSlot|GetBoardSlotOppositeBoard _returnvalue_2))
  (bind _returnvalue_4 (Class|TCBoardSlot|GetBoardSlotBoard _returnvalue_3))
  (bind _returnvalue_5 (Class|TCBoard|GetBoardSlots _returnvalue_4))
  (bind _returnvalue_6 (Class|TCBoardSlot|GetBoardSlotBoard _returnvalue_2))
  (bind _returnvalue_7 (Class|TCBoard|GetBoardSlots _returnvalue_6))
  (for (_ _array_index) _returnvalue_7
    (switch Utilities|FlowControl|Switch|SwitchonETC_TargetType (Variables|Default|GetTargetType)
      (:Self
        (CallFunction|SelfLogic))
      (:Ally
        (CallFunction|AllyLogic Caster (Utilities|Array|Get(acopy) _returnvalue_7 _array_index) (Utilities|Array|Get(acopy) _returnvalue_5 _array_index)))
      (:Enemy
        (CallFunction|EnemyLogic Caster (Utilities|Array|Get(acopy) _returnvalue_7 _array_index) (Utilities|Array|Get(acopy) _returnvalue_5 _array_index)))
      (:AllExceptSelf
        (CallFunction|AllExceptSelfLogic Caster (Utilities|Array|Get(acopy) _returnvalue_7 _array_index) (Utilities|Array|Get(acopy) _returnvalue_5 _array_index)))
      (:All
        (CallFunction|AllLogic Caster (Utilities|Array|Get(acopy) _returnvalue_7 _array_index) (Utilities|Array|Get(acopy) _returnvalue_5 _array_index))))))

(fn SelfLogic)

(fn EnemyLogic
  (params (Caster :type TC%20Card%20Object%20Reference) (AllyBoardSlot :type TC%20Board%20Slot%20Object%20Reference) (EnemyBoardSlot :type TC%20Board%20Slot%20Object%20Reference) (AllyBoard :type TC%20Board%20Object%20Reference) (EnemyBoard :type TC%20Board%20Object%20Reference) (AllyPlayerHand :type Array%20of%20TC%20Card%20Object%20References) (EnemyPlayerHand :type Array%20of%20TC%20Card%20Object%20References))
  (Utilities|IsValid EnemyBoardSlot
    (:Is%20Valid
      (bind _returnvalue (Class|TCBoardSlot|GetBoardSlotSlots EnemyBoardSlot))
      (for _array_element _returnvalue
        (bind _returnvalue_2 (Class|TCSlot|GetSlotCard _array_element))
        (Utilities|IsValid _returnvalue_2
          (:Is%20Valid
            (bind _returnvalue_3 (Class|TCCard|GetCardAttribute _returnvalue_2))
            (bind _array_element_2 (Utilities|Array|ForEachLoopwithBreak _returnvalue_3 :!label _label)
              (:LoopBody
                (if (Utilities|Array|ContainsItem (Variables|Default|GetTargetCardAttribute) _array_element_2)
                  (goto _label Break)))
              (:Completed
                (for _array_element_3 (Variables|Default|GetDataType)
                  (switch Utilities|FlowControl|Switch|SwitchonETC_DataType (.DataType (Utilities|Struct|BreakTC_DataTypeStruct _array_element_3))
                    (:Score
                      (bind _returnvalue_4 (Class|TCCard|GetCardCurrentScore _returnvalue_2))
                      (Class|TCCard|SetCardCurrentScore _returnvalue_2 (- _returnvalue_4 (Math|Conversions|ToFloat(Byte) (.StatValue (Utilities|Struct|BreakTC_DataTypeStruct _array_element_3))))))
                    (:Mana
                      (bind _returnvalue_5 (Class|TCCard|GetCardCurrentMana _returnvalue_2))
                      (Class|TCCard|SetCardCurrentMana _returnvalue_2 (- _returnvalue_5 (Math|Conversions|ToFloat(Byte) (.StatValue (Utilities|Struct|BreakTC_DataTypeStruct _array_element_3)))))))))))))
      (return))
    (:Is%20Not%20Valid
      (Utilities|IsValid EnemyBoard
        (:Is%20Valid
          (bind _returnvalue_6 (Class|TCBoard|GetBoardSlots EnemyBoard))
          (for _array_element_4 _returnvalue_6
            (bind _returnvalue_7 (Class|TCBoardSlot|GetBoardSlotSlots _array_element_4))
            (for _array_element_5 _returnvalue_7
              (bind _returnvalue_8 (Class|TCSlot|GetSlotCard _array_element_5))
              (bind _returnvalue_9 (Class|TCCard|GetCardAttribute _returnvalue_8))
              (bind _array_element_6 (Utilities|Array|ForEachLoopwithBreak _returnvalue_9 :!label _label_2)
                (:LoopBody
                  (if (Utilities|Array|ContainsItem (Variables|Default|GetTargetCardAttribute) _array_element_6)
                    (goto _label_2 Break)))
                (:Completed
                  (for _array_element_7 (Variables|Default|GetDataType)
                    (switch Utilities|FlowControl|Switch|SwitchonETC_DataType (.DataType (Utilities|Struct|BreakTC_DataTypeStruct _array_element_7))
                      (:Score
                        (bind _returnvalue_10 (Class|TCCard|GetCardCurrentScore _returnvalue_8))
                        (Class|TCCard|SetCardCurrentScore _returnvalue_8 (- _returnvalue_10 (Math|Conversions|ToFloat(Byte) (.StatValue (Utilities|Struct|BreakTC_DataTypeStruct _array_element_7))))))
                      (:Mana
                        (bind _returnvalue_11 (Class|TCCard|GetCardCurrentMana _returnvalue_8))
                        (Class|TCCard|SetCardCurrentMana _returnvalue_8 (- _returnvalue_11 (Math|Conversions|ToFloat(Byte) (.StatValue (Utilities|Struct|BreakTC_DataTypeStruct _array_element_7)))))))))))))
        (:Is%20Not%20Valid
          (if (> (Utilities|Array|Length EnemyPlayerHand) 0)
            (for _array_element_8 EnemyPlayerHand
              (Utilities|IsValid _array_element_8
                (:Is%20Valid
                  (bind _returnvalue_12 (Class|TCCard|GetCardAttribute _array_element_8))
                  (bind _array_element_9 (Utilities|Array|ForEachLoopwithBreak _returnvalue_12 :!label _label_3)
                    (:LoopBody
                      (if (Utilities|Array|ContainsItem (Variables|Default|GetTargetCardAttribute) _array_element_9)
                        (goto _label_3 Break)))
                    (:Completed
                      (for _array_element_10 (Variables|Default|GetDataType)
                        (switch Utilities|FlowControl|Switch|SwitchonETC_DataType (.DataType (Utilities|Struct|BreakTC_DataTypeStruct _array_element_10))
                          (:Score
                            (bind _returnvalue_13 (Class|TCCard|GetCardCurrentScore _array_element_8))
                            (Class|TCCard|SetCardCurrentScore _array_element_8 (- _returnvalue_13 (Math|Conversions|ToFloat(Byte) (.StatValue (Utilities|Struct|BreakTC_DataTypeStruct _array_element_10))))))
                          (:Mana
                            (bind _returnvalue_14 (Class|TCCard|GetCardCurrentMana _array_element_8))
                            (Class|TCCard|SetCardCurrentMana _array_element_8 (- _returnvalue_14 (Math|Conversions|ToFloat(Byte) (.StatValue (Utilities|Struct|BreakTC_DataTypeStruct _array_element_10)))))))))))))))))))

(fn AllExceptSelfLogic
  (params (Caster :type TC%20Card%20Object%20Reference) (AllyBoardSlot :type TC%20Board%20Slot%20Object%20Reference) (EnemyBoardSlot :type TC%20Board%20Slot%20Object%20Reference) (AllyBoard :type TC%20Board%20Object%20Reference) (EnemyBoard :type TC%20Board%20Object%20Reference) (AllyPlayerHand :type Array%20of%20TC%20Card%20Object%20References) (EnemyPlayerHand :type Array%20of%20TC%20Card%20Object%20References))
  (bind _returnvalue (Class|TCBoardSlot|GetBoardSlotSlots AllyBoardSlot))
  (for _array_element _returnvalue
    (bind _returnvalue_2 (Class|TCSlot|GetSlotCard _array_element))
    (Utilities|IsValid _returnvalue_2
      (:Is%20Valid
        (if (!= _returnvalue_2 Caster)
          (bind _returnvalue_3 (Class|TCCard|GetCardAttribute _returnvalue_2))
          (bind _array_element_2 (Utilities|Array|ForEachLoopwithBreak _returnvalue_3 :!label _label)
            (:LoopBody
              (if (Utilities|Array|ContainsItem (Variables|Default|GetTargetCardAttribute) _array_element_2)
                (goto _label Break)))
            (:Completed
              (for _array_element_3 (Variables|Default|GetDataType)
                (switch Utilities|FlowControl|Switch|SwitchonETC_DataType (.DataType (Utilities|Struct|BreakTC_DataTypeStruct _array_element_3))
                  (:Score
                    (bind _returnvalue_4 (Class|TCCard|GetCardCurrentScore _returnvalue_2))
                    (Class|TCCard|SetCardCurrentScore _returnvalue_2 (- _returnvalue_4 (Math|Conversions|ToFloat(Byte) (.StatValue (Utilities|Struct|BreakTC_DataTypeStruct _array_element_3))))))
                  (:Mana
                    (bind _returnvalue_5 (Class|TCCard|GetCardCurrentMana _returnvalue_2))
                    (Class|TCCard|SetCardCurrentMana _returnvalue_2 (- _returnvalue_5 (Math|Conversions|ToFloat(Byte) (.StatValue (Utilities|Struct|BreakTC_DataTypeStruct _array_element_3))))))))))))))
  (bind _returnvalue_6 (Class|TCBoardSlot|GetBoardSlotSlots EnemyBoardSlot))
  (for _array_element_4 _returnvalue_6
    (bind _returnvalue_7 (Class|TCSlot|GetSlotCard _array_element_4))
    (Utilities|IsValid _returnvalue_7
      (:Is%20Valid
        (bind _returnvalue_8 (Class|TCCard|GetCardAttribute _returnvalue_7))
        (bind _array_element_5 (Utilities|Array|ForEachLoopwithBreak _returnvalue_8 :!label _label_2)
          (:LoopBody
            (if (Utilities|Array|ContainsItem (Variables|Default|GetTargetCardAttribute) _array_element_5)
              (goto _label_2 Break)))
          (:Completed
            (for _array_element_6 (Variables|Default|GetDataType)
              (switch Utilities|FlowControl|Switch|SwitchonETC_DataType (.DataType (Utilities|Struct|BreakTC_DataTypeStruct _array_element_6))
                (:Score
                  (bind _returnvalue_9 (Class|TCCard|GetCardCurrentScore _returnvalue_7))
                  (Class|TCCard|SetCardCurrentScore _returnvalue_7 (- _returnvalue_9 (Math|Conversions|ToFloat(Byte) (.StatValue (Utilities|Struct|BreakTC_DataTypeStruct _array_element_6))))))
                (:Mana
                  (bind _returnvalue_10 (Class|TCCard|GetCardCurrentMana _returnvalue_7))
                  (Class|TCCard|SetCardCurrentMana _returnvalue_7 (- _returnvalue_10 (Math|Conversions|ToFloat(Byte) (.StatValue (Utilities|Struct|BreakTC_DataTypeStruct _array_element_6)))))))))))))
  (return))

(fn AllLogic
  (params (Caster :type TC%20Card%20Object%20Reference) (AllyBoardSlot :type TC%20Board%20Slot%20Object%20Reference) (EnemyBoardSlot :type TC%20Board%20Slot%20Object%20Reference) (AllyBoard :type TC%20Board%20Object%20Reference) (EnemyBoard :type TC%20Board%20Object%20Reference) (AllyPlayerHand :type Array%20of%20TC%20Card%20Object%20References) (EnemyPlayerHand :type Array%20of%20TC%20Card%20Object%20References))
  (bind _returnvalue (Class|TCBoardSlot|GetBoardSlotSlots AllyBoardSlot))
  (for _array_element _returnvalue
    (bind _returnvalue_2 (Class|TCSlot|GetSlotCard _array_element))
    (Utilities|IsValid _returnvalue_2
      (:Is%20Valid
        (bind _returnvalue_3 (Class|TCCard|GetCardAttribute _returnvalue_2))
        (bind _array_element_2 (Utilities|Array|ForEachLoopwithBreak _returnvalue_3 :!label _label)
          (:LoopBody
            (if (Utilities|Array|ContainsItem (Variables|Default|GetTargetCardAttribute) _array_element_2)
              (goto _label Break)))
          (:Completed
            (for _array_element_3 (Variables|Default|GetDataType)
              (switch Utilities|FlowControl|Switch|SwitchonETC_DataType (.DataType (Utilities|Struct|BreakTC_DataTypeStruct _array_element_3))
                (:Score
                  (bind _returnvalue_4 (Class|TCCard|GetCardCurrentScore _returnvalue_2))
                  (Class|TCCard|SetCardCurrentScore _returnvalue_2 (- _returnvalue_4 (Math|Conversions|ToFloat(Byte) (.StatValue (Utilities|Struct|BreakTC_DataTypeStruct _array_element_3))))))
                (:Mana
                  (bind _returnvalue_5 (Class|TCCard|GetCardCurrentMana _returnvalue_2))
                  (Class|TCCard|SetCardCurrentMana _returnvalue_2 (- _returnvalue_5 (Math|Conversions|ToFloat(Byte) (.StatValue (Utilities|Struct|BreakTC_DataTypeStruct _array_element_3)))))))))))))
  (bind _returnvalue_6 (Class|TCBoardSlot|GetBoardSlotSlots EnemyBoardSlot))
  (for _array_element_4 _returnvalue_6
    (bind _returnvalue_7 (Class|TCSlot|GetSlotCard _array_element_4))
    (Utilities|IsValid _returnvalue_7
      (:Is%20Valid
        (bind _returnvalue_8 (Class|TCCard|GetCardAttribute _returnvalue_7))
        (bind _array_element_5 (Utilities|Array|ForEachLoopwithBreak _returnvalue_8 :!label _label_2)
          (:LoopBody
            (if (Utilities|Array|ContainsItem (Variables|Default|GetTargetCardAttribute) _array_element_5)
              (goto _label_2 Break)))
          (:Completed
            (for _array_element_6 (Variables|Default|GetDataType)
              (switch Utilities|FlowControl|Switch|SwitchonETC_DataType (.DataType (Utilities|Struct|BreakTC_DataTypeStruct _array_element_6))
                (:Score
                  (bind _returnvalue_9 (Class|TCCard|GetCardCurrentScore _returnvalue_7))
                  (Class|TCCard|SetCardCurrentScore _returnvalue_7 (- _returnvalue_9 (Math|Conversions|ToFloat(Byte) (.StatValue (Utilities|Struct|BreakTC_DataTypeStruct _array_element_6))))))
                (:Mana
                  (bind _returnvalue_10 (Class|TCCard|GetCardCurrentMana _returnvalue_7))
                  (Class|TCCard|SetCardCurrentMana _returnvalue_7 (- _returnvalue_10 (Math|Conversions|ToFloat(Byte) (.StatValue (Utilities|Struct|BreakTC_DataTypeStruct _array_element_6)))))))))))))
  (return))

(fn TargetLogic
  (params (Caster :type TC%20Card%20Object%20Reference) (Target :type TC%20Card%20Object%20Reference))
  (Utilities|IsValid Target
    (:Is%20Valid
      (for _array_element (Variables|Default|GetDataType)
        (switch Utilities|FlowControl|Switch|SwitchonETC_DataType (.DataType (Utilities|Struct|BreakTC_DataTypeStruct _array_element))
          (:Score
            (bind _returnvalue (Class|TCCard|GetCardCurrentScore Caster))
            (Class|TCCard|SetCardCurrentScore Caster (- _returnvalue (Math|Conversions|ToFloat(Byte) (.StatValue (Utilities|Struct|BreakTC_DataTypeStruct _array_element))))))
          (:Mana
            (bind _returnvalue_2 (Class|TCCard|GetCardCurrentMana Caster))
            (Class|TCCard|SetCardCurrentMana Caster (- (Math|Conversions|ToFloat(Byte) (.StatValue (Utilities|Struct|BreakTC_DataTypeStruct _array_element))) _returnvalue_2))))))))

(fn PlayerHandLogic
  (params (Caster :type TC%20Card%20Object%20Reference)))

(fn PlayerLogic
  (params (Caster :type TC%20Card%20Object%20Reference)))

(fn BoardSlot
  (params (Caster :type TC%20Card%20Object%20Reference)))