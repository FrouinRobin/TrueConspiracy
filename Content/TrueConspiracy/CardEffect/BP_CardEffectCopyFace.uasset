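; BP_CardEffectCopyFace is a card effect that makes the caster copy the current face of a random card on the opposite board.
; On Activate, it goes from the caster's slot to the opposite board, then randomly picks a board slot and a slot within it.
; If the occupancy check passes, the caster takes that card's face.
; The check and card lookup roll random indices separately, so they can hit different slots.
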(event EventActivate
  (params (Caster :type TC%20Card%20Object%20Reference))
  (bind _returnvalue (Class|TCCard|GetSlot Caster))
  (bind _returnvalue_2 (Class|TCSlot|GetSlotBoardSlot _returnvalue))
  (bind _returnvalue_3 (Class|TCBoardSlot|GetBoardSlotOppositeBoard _returnvalue_2))
  (bind _returnvalue_4 (Class|TCBoardSlot|GetBoardSlotBoard _returnvalue_3))
  (bind _returnvalue_5 (Class|TCBoard|GetBoardSlots _returnvalue_4))
  (bind _returnvalue_6 (Class|TCBoardSlot|GetBoardSlotSlots (Utilities|Array|Get(acopy) _returnvalue_5 (Math|Random|RandomInteger (Utilities|Array|Length _returnvalue_5)))))
  (bind _returnvalue_7 (Class|TCSlot|HasCard (Utilities|Array|Get(acopy) _returnvalue_6 (Math|Random|RandomInteger (Utilities|Array|Length _returnvalue_6)))))
  (if _returnvalue_7
    (bind _returnvalue_8 (Class|TCSlot|GetSlotCard (Utilities|Array|Get(acopy) _returnvalue_6 (Math|Random|RandomInteger (Utilities|Array|Length _returnvalue_6)))))
    (bind _returnvalue_9 (Class|TCCard|GetCardCurrentFace _returnvalue_8))
    (Class|TCCard|SetCardCurrentFace Caster _returnvalue_9)))