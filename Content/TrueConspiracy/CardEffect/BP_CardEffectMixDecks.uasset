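; BP_CardEffectMixDecks is a card effect that shuffles player decks, with logic per target type.
; Ally and Enemy logic validate their input, shuffle that player's deck through the board's ShuffleCard and store the result with SetPlayerDeck.
; Plate logic does this for Player Two, then shuffles the caster's deck without storing the returned value.
; All logic only fetches Player Two's board and deck, shuffling nothing.
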(fn AllyLogic
  (params (Target :type TC%20Card%20Object%20Reference))
  (Utilities|IsValid Target
    (:Is%20Valid
      (bind _returnvalue (Class|TCCard|GetPlayer Target))
      (bind _returnvalue_2 (Class|TCPlayer|GetDeck _returnvalue))
      (bind _returnvalue_3 (Class|TCPlayer|GetPlayerBoard _returnvalue))
      (bind _returnvalue_4 (Class|TCBoard|ShuffleCard _returnvalue_3 _returnvalue_2))
      (Class|TCPlayer|SetPlayerDeck _returnvalue _returnvalue_4))))

(fn EnemyLogic
  (params (EnemyBoard :type TC%20Board%20Object%20Reference))
  (Utilities|IsValid EnemyBoard
    (:Is%20Valid
      (bind _returnvalue (Class|TCBoard|GetBoardPlayer EnemyBoard))
      (bind _returnvalue_2 (Class|TCPlayer|GetDeck _returnvalue))
      (bind _returnvalue_3 (Class|TCBoard|ShuffleCard EnemyBoard _returnvalue_2))
      (Class|TCPlayer|SetPlayerDeck _returnvalue _returnvalue_3))))

(fn PlateLogic
  (params (Caster :type TC%20Card%20Object%20Reference))
  (bind _returnvalue (Class|TCCard|GetPlayer Caster))
  (bind _returnvalue_2 (Class|TCPlayer|GetPlayerBoard _returnvalue))
  (bind _returnvalue_3 (Class|TCBoard|GetBoardPlate _returnvalue_2))
  (bind _returnvalue_4 (Class|TCPlate|GetPlayerTwo _returnvalue_3))
  (bind _returnvalue_5 (Class|TCPlayer|GetPlayerBoard _returnvalue_4))
  (bind _returnvalue_6 (Class|TCPlayer|GetDeck _returnvalue_4))
  (bind _returnvalue_7 (Class|TCBoard|ShuffleCard _returnvalue_5 _returnvalue_6))
  (Class|TCPlayer|SetPlayerDeck _returnvalue_4 _returnvalue_7)
  (bind _returnvalue_8 (Class|TCPlayer|GetDeck _returnvalue))
  (Class|TCBoard|ShuffleCard _returnvalue_2 _returnvalue_8))

(fn AllLogic
  (params (AllyBoard :type TC%20Board%20Object%20Reference) (EnemyBoard :type TC%20Board%20Object%20Reference))
  (bind _returnvalue (Class|TCBoard|GetBoardPlate AllyBoard))
  (bind _returnvalue_2 (Class|TCPlate|GetPlayerTwo _returnvalue))
  (Class|TCPlayer|GetPlayerBoard _returnvalue_2)
  (Class|TCPlayer|GetDeck _returnvalue_2))