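; AI Virus card effect that adjusts the caster's score based on Technologie cards in play.
; AllyLogic and EnemyLogic scan every slot of their respective board, counting Technologie cards other than the caster.
; Each ally match raises the score on the caster's current face by two, while each enemy match lowers that same score by two.
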(fn AllyLogic
  (params (Caster :type TC%20Card%20Object%20Reference) (AllyBoardSlot :type TC%20Board%20Slot%20Object%20Reference) (EnemyBoardSlot :type TC%20Board%20Slot%20Object%20Reference) (AllyBoard :type TC%20Board%20Object%20Reference) (EnemyBoard :type TC%20Board%20Object%20Reference) (AllyPlayerHand :type Array%20of%20TC%20Card%20Object%20References) (EnemyPlayerHand :type Array%20of%20TC%20Card%20Object%20References))
  (Utilities|IsValid AllyBoard
    (:Is%20Valid
      (Utilities|FlowControl|Sequence
        (:then_0
          (bind _returnvalue (Class|TCBoard|GetBoardSlots AllyBoard))
          (for _array_element _returnvalue
            (bind _returnvalue_2 (Class|TCBoardSlot|GetBoardSlotSlots _array_element))
            (for _array_element_2 _returnvalue_2
              (bind _returnvalue_3 (Class|TCSlot|GetSlotCard _array_element_2))
              (Utilities|IsValid _returnvalue_3
                (:Is%20Valid
                  (if (!= _returnvalue_3 Caster)
                    (bind _returnvalue_4 (Class|TCCard|GetCardAttribute _returnvalue_3))
                    (if (Utilities|Array|ContainsItem _returnvalue_4 "Technologie")
                      (Math|Integer|IncrementInt (LocalVariables|GettechnoCardsNb)))))))))
        (:then_1
          (bind _returnvalue_5 (Class|TCCard|GetCardCurrentFace Caster))
          (bind _returnvalue_6 (Class|TCFace|GetCardScore _returnvalue_5))
          (Class|TCFace|SetCardScore _returnvalue_5 (+ _returnvalue_6 (* 2 (LocalVariables|GettechnoCardsNb))))
          (return))))))

(fn EnemyLogic
  (params (Caster :type TC%20Card%20Object%20Reference) (AllyBoardSlot :type TC%20Board%20Slot%20Object%20Reference) (EnemyBoardSlot :type TC%20Board%20Slot%20Object%20Reference) (AllyBoard :type TC%20Board%20Object%20Reference) (EnemyBoard :type TC%20Board%20Object%20Reference) (AllyPlayerHand :type Array%20of%20TC%20Card%20Object%20References) (EnemyPlayerHand :type Array%20of%20TC%20Card%20Object%20References))
  (Utilities|IsValid EnemyBoard
    (:Is%20Valid
      (Utilities|FlowControl|Sequence
        (:then_0
          (bind _returnvalue (Class|TCBoard|GetBoardSlots EnemyBoard))
          (for _array_element _returnvalue
            (bind _returnvalue_2 (Class|TCBoardSlot|GetBoardSlotSlots _array_element))
            (for _array_element_2 _returnvalue_2
              (bind _returnvalue_3 (Class|TCSlot|GetSlotCard _array_element_2))
              (Utilities|IsValid _returnvalue_3
                (:Is%20Valid
                  (if (!= _returnvalue_3 Caster)
                    (bind _returnvalue_4 (Class|TCCard|GetCardAttribute _returnvalue_3))
                    (if (Utilities|Array|ContainsItem _returnvalue_4 "Technologie")
                      (Math|Integer|IncrementInt (LocalVariables|GettechnoCardsNb)))))))))
        (:then_1
          (bind _returnvalue_5 (Class|TCCard|GetCardCurrentFace Caster))
          (bind _returnvalue_6 (Class|TCFace|GetCardScore _returnvalue_5))
          (Class|TCFace|SetCardScore _returnvalue_5 (- _returnvalue_6 (* 2 (LocalVariables|GettechnoCardsNb))))
          (return))))))