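; Police card effect that adjusts the caster card's mana cost based on Gouvernement cards in the ally hand.
; AllyLogic counts its calls and, for each matching card, applies every Mana entry in DataType to the caster's current mana.
; The first call subtracts the value, the second adds it using the hand as it then stands, and later calls do nothing.
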(fn AllyLogic
  (params (Caster :type TC%20Card%20Object%20Reference) (AllyBoardSlot :type TC%20Board%20Slot%20Object%20Reference) (EnemyBoardSlot :type TC%20Board%20Slot%20Object%20Reference) (AllyBoard :type TC%20Board%20Object%20Reference) (EnemyBoard :type TC%20Board%20Object%20Reference) (AllyPlayerHand :type Array%20of%20TC%20Card%20Object%20References) (EnemyPlayerHand :type Array%20of%20TC%20Card%20Object%20References))
  (bind _result (Math|Integer|IncrementInt (Variables|Default|GetCalledInteration))
    (:%20%20
      (if (< _result 3)
        (for _array_element AllyPlayerHand
          (bind _returnvalue (Class|TCCard|GetCardAttribute _array_element))
          (if (Utilities|Array|ContainsItem _returnvalue "Gouvernement")
            (bind _array_element_2 (Utilities|Array|ForEachLoopwithBreak (Variables|Default|GetDataType))
              (:LoopBody
                (switch Utilities|FlowControl|Switch|SwitchonETC_DataType (.DataType (Utilities|Struct|BreakTC_DataTypeStruct _array_element_2))
                  (:Mana
                    (if (== (Variables|Default|GetCalledInteration) 1)
                      (bind _returnvalue_2 (Class|TCCard|GetCardCurrentMana Caster))
                      (Class|TCCard|SetCardCurrentMana Caster (- _returnvalue_2 (.StatValue (Utilities|Struct|BreakTC_DataTypeStruct _array_element_2))))
                      (else
                        (bind _returnvalue_3 (Class|TCCard|GetCardCurrentMana Caster))
                        (Class|TCCard|SetCardCurrentMana Caster (+ _returnvalue_3 (.StatValue (Utilities|Struct|BreakTC_DataTypeStruct _array_element_2))))))))))))))))