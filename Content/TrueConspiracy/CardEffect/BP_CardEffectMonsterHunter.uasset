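; Monster Hunter card effect whose EnemyLogic targets monster cards on the enemy board, apparently to send a random one back to its owner's deck.
; It collects slotted cards with the Monstre attribute into MonsterList, which is not cleared here.
; The board's player then gets a card class added to deck and a card removed from hand.
; Each call rolls its own random index, with an inclusive maximum equal to list length.
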(fn EnemyLogic
  (params (Caster :type TC%20Card%20Object%20Reference) (AllyBoardSlot :type TC%20Board%20Slot%20Object%20Reference) (EnemyBoardSlot :type TC%20Board%20Slot%20Object%20Reference) (AllyBoard :type TC%20Board%20Object%20Reference) (EnemyBoard :type TC%20Board%20Object%20Reference) (AllyPlayerHand :type Array%20of%20TC%20Card%20Object%20References) (EnemyPlayerHand :type Array%20of%20TC%20Card%20Object%20References))
  (bind _monsterlist (LocalVariables|GetMonsterList))
  (bind _returnvalue (Utilities|Array|Length _monsterlist))
  (bind _returnvalue_2 (Math|Random|RandomIntegerinRange 0 _returnvalue))
  (bind _output (Utilities|Array|Get(acopy) _monsterlist _returnvalue_2))
  (Utilities|IsValid EnemyBoard
    (:Is%20Valid
      (Utilities|FlowControl|Sequence
        (:then_0
          (for _array_element (Class|TCBoard|GetAllSlots EnemyBoard)
            (bind _returnvalue_3 (Class|TCSlot|HasCard _array_element))
            (if _returnvalue_3
              (bind _returnvalue_4 (Class|TCSlot|GetSlotCard _array_element))
              (bind _returnvalue_5 (Class|TCCard|GetCardAttribute _returnvalue_4))
              (if (Utilities|Array|ContainsItem _returnvalue_5 "Monstre")
                (Utilities|Array|Add (LocalVariables|GetMonsterList) _returnvalue_4)))))
        (:then_1
          (bind _returnvalue_6 (Class|TCBoard|GetBoardPlayer EnemyBoard))
          (Class|TCPlayer|AddCardtoDeck _returnvalue_6 (Utilities|GetClass _output))
          (Class|TCPlayer|RemoveCardfromHand _returnvalue_6 _output))))))