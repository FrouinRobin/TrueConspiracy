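; BP_CardEffectGhostBuster is a card effect that lowers the casting card's score for Apparition cards on its owner's board.
; TargetLogic scans every slot of the caster's player board and counts occupied cards with the Apparition attribute, then subtracts one point per match from the caster's current score.
; The Target only gates execution through a validity check, and the graph never resets ApparitionsCount before counting.
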(fn TargetLogic
  (params (Caster :type TC%20Card%20Object%20Reference) (Target :type TC%20Card%20Object%20Reference))
  (Utilities|IsValid Target
    (:Is%20Valid
      (Utilities|FlowControl|Sequence
        (:then_0
          (bind _returnvalue (Class|TCCard|GetPlayer Caster))
          (bind _returnvalue_2 (Class|TCPlayer|GetPlayerBoard _returnvalue))
          (for _array_element (Class|TCBoard|GetAllSlots _returnvalue_2)
            (bind _returnvalue_3 (Class|TCSlot|HasCard _array_element))
            (if _returnvalue_3
              (bind _returnvalue_4 (Class|TCSlot|GetSlotCard _array_element))
              (bind _returnvalue_5 (Class|TCCard|GetCardAttribute _returnvalue_4))
              (if (Utilities|Array|ContainsItem _returnvalue_5 "Apparition")
                (Math|Integer|IncrementInt (LocalVariables|GetApparitionsCount))))))
        (:then_1
          (bind _returnvalue_6 (Class|TCCard|GetCardCurrentScore Caster))
          (Class|TCCard|SetCardCurrentScore Caster (- _returnvalue_6 (* 1 (LocalVariables|GetApparitionsCount)))))))))