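; Card effect for the Vatican card that shuffles decks when activated by a caster.
; Activate first resolves the caster's board player through its player board, shuffles that deck via the board's ShuffleCard and sets the result back.
; It then does the same for the board plate's Player Two, a fixed slot rather than an opponent resolved relative to the caster.
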(event EventActivate
  (params (Caster :type TC%20Card%20Object%20Reference))
  (bind _returnvalue (Class|TCCard|GetPlayer Caster))
  (bind _returnvalue_2 (Class|TCPlayer|GetPlayerBoard _returnvalue))
  (Utilities|FlowControl|Sequence
    (:then_0
      (bind _returnvalue_3 (Class|TCBoard|GetBoardPlayer _returnvalue_2))
      (bind _returnvalue_4 (Class|TCPlayer|GetDeck _returnvalue_3))
      (bind _returnvalue_5 (Class|TCBoard|ShuffleCard _returnvalue_2 _returnvalue_4))
      (Class|TCPlayer|SetPlayerDeck _returnvalue_3 _returnvalue_5))
    (:then_1
      (bind _returnvalue_6 (Class|TCBoard|GetBoardPlate _returnvalue_2))
      (bind _returnvalue_7 (Class|TCPlate|GetPlayerTwo _returnvalue_6))
      (bind _returnvalue_8 (Class|TCPlayer|GetPlayerBoard _returnvalue_7))
      (bind _returnvalue_9 (Class|TCPlayer|GetDeck _returnvalue_7))
      (bind _returnvalue_10 (Class|TCBoard|ShuffleCard _returnvalue_8 _returnvalue_9))
      (Class|TCPlayer|SetPlayerDeck _returnvalue_7 _returnvalue_10))))