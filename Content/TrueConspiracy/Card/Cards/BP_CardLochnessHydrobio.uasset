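; Lochness Hydrobio card actor with attack and defend faces, each showing its illustration and a data-table-driven info widget.
; Turn, phase, placement and action events find the current face's matching effect and run it if allowed.
; Effects lacking a required target queue the card with the player and controller, though WaitingEffect is always set to the on-place type.
; Rotation flips the card anchor half a turn on a timeline.
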(event Custom|Event%20OnAction
  (bind _returnvalue (Class|TCCard|CanDoEffect))
  (if _returnvalue
    (bind _returnvalue_2 (Class|TCCard|GetCardCurrentFace))
    (bind _returnvalue_3 (Class|TCFace|FindEffectOfType _returnvalue_2 (Variables|/Script/TrueConspiracy.TC_Face|GetFaceEffect _returnvalue_2) "/Game/TrueConspiracy/EffectType/BP_EffectTypeBase.BP_EffectTypeBase_C"))
    (Utilities|IsValid _returnvalue_3
      (:Is%20Valid
        (if (CallFunction|IsSelectingTargetNeeded _returnvalue_3)
          (CallFunction|AddCardtoTargetWaitList "/Game/TrueConspiracy/EffectType/BP_EffectTypeBase.BP_EffectTypeBase_C")
          (else
            (Class|TCEffectType|DoEffect _returnvalue_3 self)))))))

(event EventBeginPlay
  (bind _returnvalue (Class|TCCard|GetCardDefendFace))
  (Class|TCCard|SetCardCurrentFace _returnvalue)
  (bind _returnvalue_2 (Class|TCCard|GetCardAttackFace))
  (Class|TCCard|AssignCardMaterialsandTextures "/Game/TrueConspiracy/FBX/Card/Materials/MI_AttackFace.MI_AttackFace" "Attack_Texture" (Variables|/Script/TrueConspiracy.TC_Face|GetFaceIllustration _returnvalue_2) "/Game/TrueConspiracy/FBX/Card/Materials/MI_DefendFace.MI_DefendFace" "Defense_Texture" (Variables|/Script/TrueConspiracy.TC_Face|GetFaceIllustration _returnvalue))
  (CallFunction|InitCardUIAttack)
  (CallFunction|InitCardUIDefense))

(event Collision|EventActorBeginOverlap
  (params (OtherActor :type Actor%20Object%20Reference)))

(event EventTick
  (params (DeltaSeconds :type Float%20%28single-precision%29)))

(event EventOnCardPlace
  (bind _returnvalue (Class|TCCard|CanDoEffect))
  (if _returnvalue
    (bind _returnvalue_2 (Class|TCCard|GetCardCurrentFace))
    (bind _returnvalue_3 (Class|TCFace|FindEffectOfType _returnvalue_2 (Variables|/Script/TrueConspiracy.TC_Face|GetFaceEffect _returnvalue_2) "/Game/TrueConspiracy/EffectType/BP_EffectTypeOnPlace.BP_EffectTypeOnPlace_C"))
    (Utilities|IsValid _returnvalue_3
      (:Is%20Valid
        (if (CallFunction|IsSelectingTargetNeeded _returnvalue_3)
          (CallFunction|AddCardtoTargetWaitList "/Game/TrueConspiracy/EffectType/BP_EffectTypeOnPlace.BP_EffectTypeOnPlace_C")
          (else
            (Class|TCEffectType|DoEffect _returnvalue_3 self)))))))

(event EventOnCardStartTurn
  (bind _returnvalue (Class|TCCard|CanDoEffect))
  (if _returnvalue
    (bind _returnvalue_2 (Class|TCCard|GetCardCurrentFace))
    (bind _returnvalue_3 (Class|TCFace|FindEffectOfType _returnvalue_2 (Variables|/Script/TrueConspiracy.TC_Face|GetFaceEffect _returnvalue_2) "/Game/TrueConspiracy/EffectType/BP_EffectTypeStartTurn.BP_EffectTypeStartTurn_C"))
    (Utilities|IsValid _returnvalue_3
      (:Is%20Valid
        (if (CallFunction|IsSelectingTargetNeeded _returnvalue_3)
          (CallFunction|AddCardtoTargetWaitList "/Game/TrueConspiracy/EffectType/BP_EffectTypeStartTurn.BP_EffectTypeStartTurn_C")
          (else
            (Class|TCEffectType|DoEffect _returnvalue_3 self)))))))

(event EventOnCardStartPhase
  (bind _returnvalue (Class|TCCard|CanDoEffect))
  (if _returnvalue
    (bind _returnvalue_2 (Class|TCCard|GetCardCurrentFace))
    (bind _returnvalue_3 (Class|TCFace|FindEffectOfType _returnvalue_2 (Variables|/Script/TrueConspiracy.TC_Face|GetFaceEffect _returnvalue_2) "/Game/TrueConspiracy/EffectType/BP_EffectTypeStartPhase.BP_EffectTypeStartPhase_C"))
    (Utilities|IsValid _returnvalue_3
      (:Is%20Valid
        (if (CallFunction|IsSelectingTargetNeeded _returnvalue_3)
          (CallFunction|AddCardtoTargetWaitList "/Game/TrueConspiracy/EffectType/BP_EffectTypeStartPhase.BP_EffectTypeStartPhase_C")
          (else
            (Class|TCEffectType|DoEffect _returnvalue_3 self)))))))

(event EventOnCardEndPhase
  (bind _returnvalue (Class|TCCard|CanDoEffect))
  (if _returnvalue
    (bind _returnvalue_2 (Class|TCCard|GetCardCurrentFace))
    (bind _returnvalue_3 (Class|TCFace|FindEffectOfType _returnvalue_2 (Variables|/Script/TrueConspiracy.TC_Face|GetFaceEffect _returnvalue_2) "/Game/TrueConspiracy/EffectType/BP_EffectTypeEndPhase.BP_EffectTypeEndPhase_C"))
    (Utilities|IsValid _returnvalue_3
      (:Is%20Valid
        (if (CallFunction|IsSelectingTargetNeeded _returnvalue_3)
          (CallFunction|AddCardtoTargetWaitList "/Game/TrueConspiracy/EffectType/BP_EffectTypeEndPhase.BP_EffectTypeEndPhase_C")
          (else
            (Class|TCEffectType|DoEffect _returnvalue_3 self)))))))

(event EventOnCardRotate
  (bind _returnvalue (Class|TCCard|GetCardAnchorRotation))
  (bind _nouvelle_piste_0 (Timeline|Chronologie PlayFromStart)
    (:Update
      (Class|TCCard|SetCardAnchorRotation (Math|Rotator|Lerp(Rotator) _returnvalue (Math|Rotator|MakeRotator (+ (.Roll (Math|Rotator|BreakRotator _returnvalue)) 1.8e+02) (.Pitch (Math|Rotator|BreakRotator _returnvalue)) (.Yaw (Math|Rotator|BreakRotator _returnvalue))) _nouvelle_piste_0)))))

(event EventOnCardEndTurn
  (bind _returnvalue (Class|TCCard|CanDoEffect))
  (if _returnvalue
    (bind _returnvalue_2 (Class|TCCard|GetCardCurrentFace))
    (bind _returnvalue_3 (Class|TCFace|FindEffectOfType _returnvalue_2 (Variables|/Script/TrueConspiracy.TC_Face|GetFaceEffect _returnvalue_2) "/Game/TrueConspiracy/EffectType/BP_EffectTypeEndTurn.BP_EffectTypeEndTurn_C"))
    (Utilities|IsValid _returnvalue_3
      (:Is%20Valid
        (if (CallFunction|IsSelectingTargetNeeded _returnvalue_3)
          (CallFunction|AddCardtoTargetWaitList "/Game/TrueConspiracy/EffectType/BP_EffectTypeEndTurn.BP_EffectTypeEndTurn_C")
          (else
            (Class|TCEffectType|DoEffect _returnvalue_3 self)))))))

(event EventOnCardSetTexture
  (bind _returnvalue (Class|TCCard|GetCardDefendFace))
  (bind _returnvalue_2 (Class|TCCard|GetCardAttackFace))
  (Class|TCCard|AssignCardMaterialsandTextures "/Game/TrueConspiracy/FBX/Card/Materials/MI_AttackFace.MI_AttackFace" "Attack_Texture" (Variables|/Script/TrueConspiracy.TC_Face|GetFaceIllustration _returnvalue_2) "/Game/TrueConspiracy/FBX/Card/Materials/MI_DefendFace.MI_DefendFace" "Defense_Texture" (Variables|/Script/TrueConspiracy.TC_Face|GetFaceIllustration _returnvalue)))

(fn ConstructionScript
  (CallFunction|InitCardUIAttack)
  (CallFunction|InitCardUIDefense))

(fn IsSelectingTargetNeeded
  (params (Effect%20Type :type TC%20Effect%20Type%20Object%20Reference))
  (return (and (Class|TCEffectType|DoesEffectRequireTarget Effect%20Type) (not (Utilities|IsValid (Class|TCEffectType|GetTarget Effect%20Type))))))

(fn AddCardtoTargetWaitList
  (params (Effect%20Type :type TC%20Effect%20Type%20Class%20Reference))
  (bind _returnvalue (Class|TCCard|GetPlayer))
  (Utilities|FlowControl|Sequence
    (:then_0
      (Class|TCPlayer|AddCardtoWaitingTargetList _returnvalue self)
      (Variables|Default|SetWaitingEffect "/Game/TrueConspiracy/EffectType/BP_EffectTypeOnPlace.BP_EffectTypeOnPlace_C"))
    (:then_1
      (bind _asbp_player_pawn (Utilities|Casting|CastToBP_PlayerPawn _returnvalue))
      (bind _asbp_player_controller (Utilities|Casting|CastToBP_PlayerController (Default|GetPawnController _asbp_player_pawn)))
      (Variables|/Game/TrueConspiracy/Player/BP_PlayerController.BP_PlayerController_C|SetCardCache _asbp_player_controller self))))

(fn InitCardUIAttack
  (bind _returnvalue (Utilities|GetDataTableRow (Variables|Default|GetCardDataTable) (Variables|Default|GetCardRowNameAttack))
    (:then
      (bind _asbp_card_info_game (Utilities|Casting|CastToBP_CardInfoGame (UserInterface|GetUserWidgetObject (Variables|Default|GetCardUIAttack))))
      (bind _output_get (Variables|/Game/TrueConspiracy/Card/BP_CardInfoGame.BP_CardInfoGame_C|SetcardData _asbp_card_info_game _returnvalue))
      (Default|SetCardInfo _asbp_card_info_game _output_get 0.0 0.0))))

(fn InitCardUIDefense
  (bind _returnvalue (Utilities|GetDataTableRow (Variables|Default|GetCardDataTable) (Variables|Default|GetCardRowNameDefense))
    (:then
      (bind _asbp_card_info_game (Utilities|Casting|CastToBP_CardInfoGame (UserInterface|GetUserWidgetObject (Variables|Default|GetCardUIDefense))))
      (bind _output_get (Variables|/Game/TrueConspiracy/Card/BP_CardInfoGame.BP_CardInfoGame_C|SetcardData _asbp_card_info_game _returnvalue))
      (Default|SetCardInfo _asbp_card_info_game _output_get 0.0 0.0))))