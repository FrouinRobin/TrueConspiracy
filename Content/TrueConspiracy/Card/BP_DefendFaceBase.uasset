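; BP_DefendFaceBase is the base Blueprint for a card's defend face, running face effects at key moments in play.
; It handles six face events: placement, turn start, turn end, each turn, phase start and phase end.
; Each handler repeats the same pattern: check the FaceEffect collection for an entry, look it up by index and call DoEffect on it.
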(event EventOnFaceEachTurn
  (bind _faceeffect (Variables|Default|GetFaceEffect))
  (if (Utilities|Array|ContainsItem (Variables|Default|GetFaceEffect) 0)
    (Class|TCEffectType|DoEffect (Utilities|Array|Get(acopy) _faceeffect (Utilities|Array|FindItem _faceeffect 0)))))

(event EventOnFaceEndPhase
  (bind _faceeffect (Variables|Default|GetFaceEffect))
  (if (Utilities|Array|ContainsItem (Variables|Default|GetFaceEffect) 0)
    (Class|TCEffectType|DoEffect (Utilities|Array|Get(acopy) _faceeffect (Utilities|Array|FindItem _faceeffect 0)))))

(event EventOnFaceEndTurn
  (bind _faceeffect (Variables|Default|GetFaceEffect))
  (if (Utilities|Array|ContainsItem (Variables|Default|GetFaceEffect) 0)
    (Class|TCEffectType|DoEffect (Utilities|Array|Get(acopy) _faceeffect (Utilities|Array|FindItem _faceeffect 0)))))

(event EventOnFacePlace
  (bind _faceeffect (Variables|Default|GetFaceEffect))
  (if (Utilities|Array|ContainsItem (Variables|Default|GetFaceEffect) 0)
    (Class|TCEffectType|DoEffect (Utilities|Array|Get(acopy) _faceeffect (Utilities|Array|FindItem _faceeffect 0)))))

(event EventOnFaceStartPhase
  (bind _faceeffect (Variables|Default|GetFaceEffect))
  (if (Utilities|Array|ContainsItem (Variables|Default|GetFaceEffect) 0)
    (Class|TCEffectType|DoEffect (Utilities|Array|Get(acopy) _faceeffect (Utilities|Array|FindItem _faceeffect 0)))))

(event EventOnFaceStartTurn
  (bind _faceeffect (Variables|Default|GetFaceEffect))
  (if (Utilities|Array|ContainsItem (Variables|Default|GetFaceEffect) 0)
    (Class|TCEffectType|DoEffect (Utilities|Array|Get(acopy) _faceeffect (Utilities|Array|FindItem _faceeffect 0)))))