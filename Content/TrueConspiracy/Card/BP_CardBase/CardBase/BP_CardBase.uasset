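; BP_CardBase is a base card Blueprint that triggers effects at card placement and at turn and phase boundaries.
; Each event checks CanDoEffect, finds an effect by type on the current face and runs DoEffect on the card.
; Turn start and turn end both look up the EndPhase type, the same as phase end.
; BeginPlay only prints the player's phase state.
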(event EventBeginPlay
  (bind _returnvalue (Class|TCCard|GetPlayer))
  (Development|PrintString (Utilities|String|EnumtoString (Variables|/Script/TrueConspiracy.TC_Player|Get_phaseState _returnvalue))))

(event Collision|EventActorBeginOverlap
  (params (OtherActor :type Actor%20Object%20Reference)))

(event EventTick
  (params (DeltaSeconds :type Float%20%28single-precision%29)))

(event EventOnCardPlace
  (bind _returnvalue (Class|TCCard|CanDoEffect))
  (if _returnvalue
    (bind _returnvalue_2 (Class|TCCard|GetCardCurrentFace))
    (bind _returnvalue_3 (Class|TCFace|FindEffectOfType _returnvalue_2 (Variables|/Script/TrueConspiracy.TC_Face|GetFaceEffect _returnvalue_2) "/Game/TrueConspiracy/EffectType/BP_EffectTypeOnPlace.BP_EffectTypeOnPlace_C"))
    (Class|TCEffectType|DoEffect _returnvalue_3 self)))

(event EventOnCardStartTurn
  (bind _returnvalue (Class|TCCard|CanDoEffect))
  (if _returnvalue
    (bind _returnvalue_2 (Class|TCCard|GetCardCurrentFace))
    (bind _returnvalue_3 (Class|TCFace|FindEffectOfType _returnvalue_2 (Variables|/Script/TrueConspiracy.TC_Face|GetFaceEffect _returnvalue_2) "/Game/TrueConspiracy/EffectType/BP_EffectTypeEndPhase.BP_EffectTypeEndPhase_C"))
    (Class|TCEffectType|DoEffect _returnvalue_3 self)))

(event EventOnCardStartPhase
  (bind _returnvalue (Class|TCCard|CanDoEffect))
  (if _returnvalue
    (bind _returnvalue_2 (Class|TCCard|GetCardCurrentFace))
    (bind _returnvalue_3 (Class|TCFace|FindEffectOfType _returnvalue_2 (Variables|/Script/TrueConspiracy.TC_Face|GetFaceEffect _returnvalue_2) "/Game/TrueConspiracy/EffectType/BP_EffectTypeStartPhase.BP_EffectTypeStartPhase_C"))
    (Class|TCEffectType|DoEffect _returnvalue_3 self)))

(event EventOnCardEndPhase
  (bind _returnvalue (Class|TCCard|CanDoEffect))
  (if _returnvalue
    (bind _returnvalue_2 (Class|TCCard|GetCardCurrentFace))
    (bind _returnvalue_3 (Class|TCFace|FindEffectOfType _returnvalue_2 (Variables|/Script/TrueConspiracy.TC_Face|GetFaceEffect _returnvalue_2) "/Game/TrueConspiracy/EffectType/BP_EffectTypeEndPhase.BP_EffectTypeEndPhase_C"))
    (Class|TCEffectType|DoEffect _returnvalue_3 self)))

(event EventOnCardEndTurn
  (bind _returnvalue (Class|TCCard|CanDoEffect))
  (if _returnvalue
    (bind _returnvalue_2 (Class|TCCard|GetCardCurrentFace))
    (bind _returnvalue_3 (Class|TCFace|FindEffectOfType _returnvalue_2 (Variables|/Script/TrueConspiracy.TC_Face|GetFaceEffect _returnvalue_2) "/Game/TrueConspiracy/EffectType/BP_EffectTypeEndPhase.BP_EffectTypeEndPhase_C"))
    (Class|TCEffectType|DoEffect _returnvalue_3 self)))

(fn ConstructionScript)