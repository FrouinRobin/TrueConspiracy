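; BP_Lochness is an attack-face card effect whose logic is currently disconnected.
; Its custom event takes a Caster and reaches only a switch on Land with no wired cases, so it changes nothing.
; Unexecuted nodes sketch a search of the board plate's land slots for the caster's slot, then a card max score boost, larger for one test card ID.
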(event Custom|CustomEvent
  (params (Caster :type TC%20Card%20Object%20Reference))
  (switch Utilities|FlowControl|Switch|SwitchonETC_EffectLocalisation "Land"))